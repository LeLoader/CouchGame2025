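; BP_CameraCine is a free-fly camera actor, judging by its name for cinematic shots, steered through three functions that other code is expected to call.
; Move translates it along its own forward and right vectors, and Lift along its up vector, both scaled by CameraSpeed.
; Look adds input to yaw and inverted input to pitch, with no clamping or delta-time scaling.
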(event EventBeginPlay)

(event Collision|EventActorBeginOverlap
  (params (OtherActor :type Actor%20Object%20Reference)))

(event EventTick
  (params (DeltaSeconds :type Float%20%28single-precision%29)))

(fn ConstructionScript)

(fn Move
  (params (X :type Float%20%28double-precision%29) (Y :type Float%20%28double-precision%29))
  (Transformation|SetActorLocation (+ (Transformation|GetActorLocation) (* (Transformation|GetActorForwardVector) Y (Variables|Default|GetCameraSpeed)) (* (Transformation|GetActorRightVector) X (Variables|Default|GetCameraSpeed))) false false))

(fn Look
  (params (X :type Float%20%28double-precision%29) (Y :type Float%20%28double-precision%29))
  (bind _returnvalue (Transformation|GetActorRotation))
  (Transformation|SetActorRotation (Math|Rotator|MakeRotator (.roll _returnvalue) (+ (.pitch _returnvalue) (* Y -1.0)) (+ X (.yaw _returnvalue)))))

(fn Lift
  (params (Value :type Float%20%28double-precision%29))
  (Transformation|SetActorLocation (+ (* (Transformation|GetActorUpVector) Value (Variables|Default|GetCameraSpeed)) (Transformation|GetActorLocation)) false false))