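; Rope constraint between the two BP_Character players, drawn as a cable and disabled at start.
; While enabled, Tick slows each player's walk speed using a distance curve scaled by how much that player faces away from the other.
; Enable and Toggle only switch it on within MaxDistance, and Disable restores speed and hides the cable.
; TeleportToOtherPlayer moves the other player to the instigator while linked.
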(event EventBeginPlay
  (bind _outactors (Actor|GetAllActorsOfClass "/Game/CouchGame2025/Blueprint/BP_Character.BP_Character_C"))
  (bind _output_get (Variables|Default|SetPlayer1 (Utilities|Array|Get(acopy) _outactors)))
  (bind _output_get_2 (Variables|Default|SetPlayer2 (Utilities|Array|Get(acopy) _outactors 1)))
  (Variables|Default|SetInitMaxWalkingSpeed (Variables|/Script/Engine.CharacterMovementComponent|GetMaxWalkSpeed (Variables|/Script/Engine.Character|GetCharacterMovement _output_get_2)))
  (Transformation|AttachActorToActor _output_get_2 "RopeSocket" "SnapToTarget" "SnapToTarget" "KeepRelative" false)
  (Class|CableComponentBis|SetAttachEndtoComponent (Variables|Default|GetCableComponentBis) (Variables|/Script/Engine.Actor|GetRootComponent _output_get) "RopeSocket")
  (CallFunction|Disable))

(event EventTick
  (params (DeltaSeconds :type Float%20%28single-precision%29))
  (bind _player1 (Variables|Default|GetPlayer1))
  (bind _player2 (Variables|Default|GetPlayer2))
  (bind _curve (Variables|Default|GetCurve))
  (bind _maxdistance (Variables|Default|GetMaxDistance))
  (bind _returnvalue (Transformation|GetActorLocation _player1))
  (bind _returnvalue_2 (Transformation|GetActorLocation _player2))
  (bind _returnvalue_3 (Math|Vector|Distance(Vector) _returnvalue _returnvalue_2))
  (bind _returnvalue_4 (/ _returnvalue_3 _maxdistance))
  (bind _returnvalue_5 (Math|Curves|GetFloatValue _curve _returnvalue_4))
  (if (Variables|Default|GetbEnabled)
    (Development|PrintString "Hello" true true "(R=0.000000,G=0.660000,B=1.000000,A=1.000000)" 2.0 "distancetovalue")
    (Variables|/Script/Engine.CharacterMovementComponent|SetMaxWalkSpeed (Variables|/Script/Engine.Character|GetCharacterMovement _player1) (Math|Float|Lerp (Variables|Default|GetInitMaxWalkingSpeed) 0.0 (* (- 1.0 (/ (+ (Math|Vector|DotProduct (Transformation|GetActorForwardVector _player1) (Math|Vector|Normalize (- (Transformation|GetActorLocation _player2) (Transformation|GetActorLocation _player1)))) 1.0) 2.0)) _returnvalue_5)))
    (Variables|/Script/Engine.CharacterMovementComponent|SetMaxWalkSpeed (Variables|/Script/Engine.Character|GetCharacterMovement _player2) (Math|Float|Lerp (Variables|Default|GetInitMaxWalkingSpeed) 0.0 (* (- 1.0 (/ (+ (Math|Vector|DotProduct (Transformation|GetActorForwardVector _player2) (Math|Vector|Normalize (- (Transformation|GetActorLocation _player1) (Transformation|GetActorLocation _player2)))) 1.0) 2.0)) _returnvalue_5)))))

(fn ConstructionScript)

(fn CanEnable
  (return (< (Math|Vector|Distance(Vector) (Transformation|GetActorLocation (Variables|Default|GetPlayer1)) (Transformation|GetActorLocation (Variables|Default|GetPlayer2))) (Variables|Default|GetMaxDistance))))

(fn Enable
  (bind _output_get (Variables|Default|SetbEnabled (CallFunction|CanEnable)))
  (Rendering|SetVisibility (Variables|Default|GetCableComponentBis) _output_get false)
  (return _output_get))

(fn Disable
  (Variables|Default|SetbEnabled false)
  (bind _output_get (Variables|/Script/Engine.CharacterMovementComponent|SetMaxWalkSpeed (Variables|/Script/Engine.Character|GetCharacterMovement (Variables|Default|GetPlayer1)) (Variables|Default|GetInitMaxWalkingSpeed)))
  (Variables|/Script/Engine.CharacterMovementComponent|SetMaxWalkSpeed (Variables|/Script/Engine.Character|GetCharacterMovement (Variables|Default|GetPlayer2)) _output_get)
  (Rendering|SetVisibility (Variables|Default|GetCableComponentBis) false false))

(fn Toggle
  (if (Variables|Default|GetbEnabled)
    (CallFunction|Disable)
    (return false)
    (else
      (bind _hasenabled (CallFunction|Enable))
      (return _hasenabled))))

(fn TeleporttoOtherPlayer
  (params (Instigator :type BP%20Character%20Object%20Reference))
  (bind _player1 (Variables|Default|GetPlayer1))
  (bind _player2 (Variables|Default|GetPlayer2))
  (if (Variables|Default|GetbEnabled)
    (if (== Instigator (Variables|Default|GetPlayer1))
      (Transformation|SetActorLocation _player2 (Transformation|GetActorLocation _player1) false true)
      (else
        (Transformation|SetActorLocation _player1 (Transformation|GetActorLocation _player2) false true)))))