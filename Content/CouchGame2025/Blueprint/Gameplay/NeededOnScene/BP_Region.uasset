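; Gameplay region that tracks objectives and transitions its meshes between frozen and alive states.
; Builds objective objects from a data table, advancing them through trash destruction, injector resource and ice seed events, filtering trash and seeds by region tag.
; Objective completion triggers a region check that broadcasts completion and enables the big bridge.
; A full injector drives a timeline updating material parameters on region, isles and props, centred via a parameter collection.
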(event Custom|OnTrashDestroyed
  (params (Trash :type Actor%20Object%20Reference))
  (if (Actor|ActorHasTag Trash (Variables|Default|GetTag))
    (Default|ProgressObjective (CallFunction|GetObjectivefromObjectiveType "NewEnumerator0") 1.0 "NewEnumerator0")))

(event Custom|OnRessourceUpdated
  (params (NewRessourceAmount :type Float%20%28single-precision%29) (OldRessourceAmount :type Float%20%28single-precision%29))
  (Default|ProgressObjective (CallFunction|GetObjectivefromObjectiveType "NewEnumerator1") (- NewRessourceAmount OldRessourceAmount) "NewEnumerator1"))

(event Custom|OnIceUnfreezed
  (Default|ProgressObjective (CallFunction|GetObjectivefromObjectiveType "NewEnumerator2") 1.0 "NewEnumerator2"))

(event Custom|CE_chose
  (Utilities|FlowControl|DoOnce false
    (:Completed
      (Rendering|Material|SetVectorParameterValue "/Game/CouchGame2025/Asset/props/materiaux/MPC_Transition.MPC_Transition" "InjectorPosition" (Math|Conversions|ToLinearColor(Vector) (Transformation|GetActorLocation (Variables|Default|GetInjector))) :!class /Script/Engine.KismetMaterialLibrary)
      (Components|Timeline|SetPlayRate (Variables|Default|GetTimeline) (/ 1.0 (Variables|Default|GetSpeed)))
      (bind _float (Timeline|Timeline PlayFromStart)
        (:Update
          (Rendering|Material|SetScalarParameterValueonMaterials (Variables|/Script/Engine.StaticMeshActor|GetStaticMeshComponent (Variables|Default|GetRegionMesh)) "Alive > Frozen" _float)
          (for _array_element (Variables|Default|GetIslesMesh)
            (Rendering|Material|SetScalarParameterValueonMaterials (Variables|/Script/Engine.StaticMeshActor|GetStaticMeshComponent _array_element) "Alive > Frozen" _float))
          (for _array_element_2 (Variables|Default|GetProps)
            (Rendering|Material|SetScalarParameterValueonMaterials _array_element_2 "Alive > Frozen" (- 1.0 _float))))))))

(event Custom|OnContainerFull
  (params (speed :type Float%20%28double-precision%29))
  (Rendering|Material|SetVectorParameterValue "/Game/CouchGame2025/Asset/props/materiaux/MPC_Transition.MPC_Transition" "InjectorPosition" (Math|Conversions|ToLinearColor(Vector) (Transformation|GetActorLocation (Variables|Default|GetInjector))) :!class /Script/Engine.KismetMaterialLibrary)
  (Components|Timeline|SetPlayRate (Variables|Default|GetTimeline) (/ 1.0 (Variables|Default|GetSpeed)))
  (bind _float (Timeline|Timeline PlayFromStart)
    (:Update
      (Rendering|Material|SetScalarParameterValueonMaterials (Variables|/Script/Engine.StaticMeshActor|GetStaticMeshComponent (Variables|Default|GetRegionMesh)) "Alive > Frozen" _float)
      (for _array_element (Variables|Default|GetIslesMesh)
        (Rendering|Material|SetScalarParameterValueonMaterials (Variables|/Script/Engine.StaticMeshActor|GetStaticMeshComponent _array_element) "Alive > Frozen" _float))
      (for _array_element_2 (Variables|Default|GetProps)
        (Rendering|Material|SetScalarParameterValueonMaterials _array_element_2 "Alive > Frozen" (- 1.0 _float))))))

(event Custom|CE_FindAllProps
  (Utilities|Array|Clear (Variables|Default|GetProps))
  (bind _outactors (Actor|GetAllActorsOfClasswithTag "/Script/Engine.StaticMeshActor" (Variables|Default|GetTag)))
  (for _array_element _outactors
    (Utilities|Array|Add (Variables|Default|GetProps) (Variables|/Script/Engine.StaticMeshActor|GetStaticMeshComponent _array_element))
    (for _array_element_2 (Components|GetChildrenComponents (Variables|/Script/Engine.StaticMeshActor|GetStaticMeshComponent _array_element) true)
      (bind _asmesh_component (Utilities|Casting|CastToMeshComponent _array_element_2))
      (Utilities|Array|Add (Variables|Default|GetProps) _asmesh_component))))

(event Custom|OnObjectiveCompleted
  (params (Type :type E_ObjectiveType%20Enum :default "NewEnumerator0"))
  (if (CallFunction|IsRegionCompleted)
    ;[0.15 0 0 0.5] Unlock next region, prob from gm
    (Default|CallOnRegionCompleted)
    (bind _returnvalue (Actor|GetActorOfClass "/Game/CouchGame2025/Blueprint/Gameplay/BP_BigBridge.BP_BigBridge_C"))
    (Rendering|SetVisibility (Variables|/Game/CouchGame2025/Blueprint/Gameplay/BP_BigBridge.BP_BigBridge_C|GetStaticMesh _returnvalue) true false)
    (Collision|SetCollisionEnabled (Variables|/Game/CouchGame2025/Blueprint/Gameplay/BP_BigBridge.BP_BigBridge_C|GetStaticMesh _returnvalue) "QueryAndPhysics")))

(event EventBeginPlay
  (EventDispatchers|AssignOnContainerFull (Variables|Default|GetInjector) (EventDispatchers|CreateEvent :!event Custom|OnContainerFull))
  (bind _outrownames (DataTable|GetDataTableRowNames (Variables|Default|GetObjectivesDataTable)))
  (for _array_element _outrownames
    (bind _returnvalue (Utilities|GetDataTableRow (Variables|Default|GetObjectivesDataTable) _array_element)
      (:then
        (bind _returnvalue_2 (Game|ConstructObjectfromClass (CallFunction|GetObjectiveClassfromObjectiveType (.Type (Utilities|Struct|BreakS_Objective _returnvalue))) (.Goal (Utilities|Struct|BreakS_Objective _returnvalue)) (.Name (Utilities|Struct|BreakS_Objective _returnvalue))))
        (Utilities|Array|Add (Variables|Default|GetObjectives) _returnvalue_2)
        (EventDispatchers|AssignOnObjectiveCompleted _returnvalue_2 (EventDispatchers|CreateEvent :!event Custom|OnObjectiveCompleted))
        (switch Utilities|FlowControl|Switch|SwitchonE_ObjectiveType (.Type (Utilities|Struct|BreakS_Objective _returnvalue))
          (:NewEnumerator0
            (bind _returnvalue_3 (Actor|GetActorOfClass "/Game/CouchGame2025/Blueprint/Gameplay/NeededOnScene/BP_BlackHole.BP_BlackHole_C"))
            (EventDispatchers|BindEventtoOnTrashDestroyed _returnvalue_3 (EventDispatchers|CreateEvent :!event Custom|OnTrashDestroyed)))
          (:NewEnumerator1
            (EventDispatchers|BindEventtoOnRessourceUpdated (Variables|/Script/CouchGame2025.RessourceInjector|GetRessourceContainer (Variables|Default|GetInjector)) (EventDispatchers|CreateEvent :!event Custom|OnRessourceUpdated)))
          (:NewEnumerator2
            (bind _outactors (Actor|GetAllActorsOfClasswithTag "/Game/CouchGame2025/Blueprint/Gameplay/BP_Iceseed.BP_Iceseed_C" (Variables|Default|GetTag)))
            (for _array_element_2 _outactors
              (EventDispatchers|AssignOnIceSeedPickable _array_element_2 (EventDispatchers|CreateEvent :!event Custom|OnIceUnfreezed)))))))))

(fn ConstructionScript)

(fn IsRegionCompleted
  (bind _array_element (Utilities|Array|ForEachLoopwithBreak (Variables|Default|GetObjectives) :!label _label)
    (:LoopBody
      (if (not (Variables|/Game/CouchGame2025/Data/Objectives/Objective.Objective_C|GetbIsCompleted _array_element))
        (goto _label Break)))
    (:Completed
      (return true))))

(fn GetObjectiveClassfromObjectiveType
  (params (ObjectiveType :type E_ObjectiveType%20Enum :default "NewEnumerator0"))
  (return (Utilities|Select :Index ObjectiveType :NewEnumerator0 "/Game/CouchGame2025/Data/Objectives/TrashObjective.TrashObjective_C" :NewEnumerator1 "/Game/CouchGame2025/Data/Objectives/InjectorObjective.InjectorObjective_C" :NewEnumerator2 "/Game/CouchGame2025/Data/Objectives/IceseedObjective.IceseedObjective_C")))

(fn GetObjectivefromObjectiveType
  (params (Type :type E_ObjectiveType%20Enum :default "NewEnumerator0"))
  (for _array_element (Variables|Default|GetObjectives)
    (if (Utilities|Enum|Equal(Enum) (Variables|/Game/CouchGame2025/Data/Objectives/Objective.Objective_C|GetType _array_element) Type)
      (return _array_element)))
  (return 0))