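; Test actor with a camera that keeps itself oriented on the world origin, apparently for polar-style movement.
; Each tick runs the parent logic, then turns the actor toward the origin, or away when inverted, and applies pitch and yaw offsets to the camera.
; The construction script previews the inward-facing orientation and camera offsets.
; A custom event sets the flag that allows movement.
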(event Custom|CE_AllowMovement
  (Variables|Default|SetcanMove true))

(event EventTick
  (params (DeltaSeconds :type Float%20%28single-precision%29))
  (bind _returnvalue (Transformation|GetActorLocation))
  (bind _returnvalue_2 (Math|Vector|MakeVector 0.0 0.0 0.0))
  (|CallParentFunction DeltaSeconds)
  (Transformation|SetActorRotation (select (Variables|Default|GetbisInverted) (Math|Rotator|FindLookatRotation _returnvalue_2 _returnvalue) (Math|Rotator|FindLookatRotation _returnvalue _returnvalue_2)))
  (Transformation|SetRelativeRotation (Variables|Default|GetCameraComponent) (Math|Rotator|MakeRotator 0.0 (Variables|Default|GetPitchOffsetValue) (Variables|Default|GetYawOffsetValue)) false false))

(fn ConstructionScript
  (Transformation|SetActorRotation (Math|Rotator|FindLookatRotation (Transformation|GetActorLocation) (Math|Vector|MakeVector 0.0 0.0 0.0)))
  (Transformation|SetRelativeRotation (Variables|Default|GetCameraComponent) (Math|Rotator|MakeRotator 0.0 (Variables|Default|GetPitchOffsetValue) (Variables|Default|GetYawOffsetValue)) false false))