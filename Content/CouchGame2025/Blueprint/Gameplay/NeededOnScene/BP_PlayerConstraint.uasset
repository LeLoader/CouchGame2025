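; Scene actor that manages the rope between two player characters through CableComponentBis.
; Toggle asks the cable to switch the rope for the instigator and prints the result.
; While the cable is visible, TeleportToOtherPlayer, despite its name, pulls the other character to the instigator's location, or the start character to the end if the instigator isn't the start.
; It then copies the planetary movement's external-gravity setting and tries toggling the rope.
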(fn ConstructionScript)

(fn TeleporttoOtherPlayer
  (params (Instigator :type BP%20Character%20Object%20Reference))
  (bind _cablecomponentbis (Variables|Default|GetCableComponentBis))
  (bind _characterstart (Variables|/Script/CableComponentBis.CableComponentBis|GetCharacterStart _cablecomponentbis))
  (bind _characterend (Variables|/Script/CableComponentBis.CableComponentBis|GetCharacterEnd _cablecomponentbis))
  (if (Rendering|IsVisible _cablecomponentbis)
    (if (== Instigator _characterstart)
      (Transformation|SetActorLocation _characterend (Transformation|GetActorLocation _characterstart) false true)
      (bind _asbp_character (Utilities|Casting|CastToBP_Character _characterstart))
      (bind _asbp_character_2 (Utilities|Casting|CastToBP_Character _characterend))
      (Variables|/Script/CouchGame2025.PlanetaryMovementComponent|SetUseExternalGravityDirection (Variables|/Game/CouchGame2025/Blueprint/BP_Character.BP_Character_C|GetPlanetary%20Movement%20Component _asbp_character_2) (Variables|/Script/CouchGame2025.PlanetaryMovementComponent|GetUseExternalGravityDirection (Variables|/Game/CouchGame2025/Blueprint/BP_Character.BP_Character_C|GetPlanetary%20Movement%20Component _asbp_character)))
      (else
        (Transformation|SetActorLocation _characterstart (Transformation|GetActorLocation _characterend) false true)
        (bind _asbp_character_3 (Utilities|Casting|CastToBP_Character _characterend))
        (bind _asbp_character_4 (Utilities|Casting|CastToBP_Character _characterstart))
        (Variables|/Script/CouchGame2025.PlanetaryMovementComponent|SetUseExternalGravityDirection (Variables|/Game/CouchGame2025/Blueprint/BP_Character.BP_Character_C|GetPlanetary%20Movement%20Component _asbp_character_4) (Variables|/Script/CouchGame2025.PlanetaryMovementComponent|GetUseExternalGravityDirection (Variables|/Game/CouchGame2025/Blueprint/BP_Character.BP_Character_C|GetPlanetary%20Movement%20Component _asbp_character_3)))))
    (Class|CableComponentBis|TryToggleRope (Variables|Default|GetCableComponentBis) Instigator)))

(fn Toggle
  (params (Instigator :type BP%20Character%20Object%20Reference))
  (bind _returnvalue (Class|CableComponentBis|TryToggleRope (Variables|Default|GetCableComponentBis) Instigator))
  (Development|PrintString (Utilities|String|ToString(Boolean) _returnvalue)))