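; Base meteor Blueprint whose pull is driven by an ObjectPlanetaryGravity component.
; BeginPlay stores the component's gravity force as the target, and Tick continuously interpolates the live force toward that target.
; AccelerateTowardGravity multiplies the target fivefold behind a DoOnce, so the meteor's gravity ramps up smoothly and only a single time.
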(event Custom|AccelerateTowardGravity
  (Utilities|FlowControl|DoOnce false
    (:Completed
      (Variables|Default|SetTargetGravity (* (Variables|Default|GetTargetGravity) 5.0)))))

(event EventBeginPlay
  (|CallParentFunction)
  (Variables|Default|SetTargetGravity (Variables|/Script/CouchGame2025.ObjectPlanetaryGravityComponent|GetGravityForce (Variables|Default|GetObjectPlanetaryGravity))))

(event Collision|EventActorBeginOverlap
  (params (OtherActor :type Actor%20Object%20Reference))
  (|CallParentFunction OtherActor) ; This node is disabled and will not be called.\nDrag off pins to build functionality.
)

(event EventTick
  (params (DeltaSeconds :type Float%20%28single-precision%29))
  (bind _objectplanetarygravity (Variables|Default|GetObjectPlanetaryGravity))
  (|CallParentFunction DeltaSeconds)
  (Variables|/Script/CouchGame2025.ObjectPlanetaryGravityComponent|SetGravityForce _objectplanetarygravity (Math|Interpolation|FInterpTo (Variables|/Script/CouchGame2025.ObjectPlanetaryGravityComponent|GetGravityForce _objectplanetarygravity) (Variables|Default|GetTargetGravity) DeltaSeconds 1.0)))

(fn ConstructionScript
  (|CallParentFunction))