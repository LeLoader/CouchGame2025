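; BP_MeteorBase1 is a meteor gameplay actor with a Niagara effect and a water capacity query.
; TriggerParticule toggles the Niagara component between active and inactive without resetting it.
; GetMaxWater always returns zero, and the MaxRessourceAmount variable is unused.
; The construction script only calls its parent, and BeginPlay, overlap and Tick are disabled placeholders.
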(event EventBeginPlay
  (|CallParentFunction) ; This node is disabled and will not be called.\nDrag off pins to build functionality.
)

(event Collision|EventActorBeginOverlap
  (params (OtherActor :type Actor%20Object%20Reference))
  (|CallParentFunction OtherActor) ; This node is disabled and will not be called.\nDrag off pins to build functionality.
)

(event EventTick
  (params (DeltaSeconds :type Float%20%28single-precision%29))
  (|CallParentFunction DeltaSeconds) ; This node is disabled and will not be called.\nDrag off pins to build functionality.
)

(event EventTriggerParticule
  (bind _niagara (Variables|Default|GetNiagara))
  (Components|Activation|SetActive _niagara (not (Components|Activation|IsActive _niagara)) false))

(fn ConstructionScript
  (|CallParentFunction))

(fn GetMaxWater
  (return 0.0))