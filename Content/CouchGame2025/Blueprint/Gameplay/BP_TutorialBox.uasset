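; Tutorial trigger volume that shows one-time dialogue when a character enters or exits its box, using lines from a data table row.
; NextDialogue binds the triggering character's OnNextDialogue event and switches all characters' Enhanced Input contexts to IMC_Dialogue.
; Talk steps through lines in WBP_Dialogue, then removes the widget, unbinds events and restores each player's device-specific context.
; GoToTalk picks entry or exit text by checking whether that character still overlaps the box.
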(event OnComponentBeginOverlap(Box)
  (params (OverlappedComponent :type Primitive%20Component%20Object%20Reference) (OtherActor :type Actor%20Object%20Reference) (OtherComp :type Primitive%20Component%20Object%20Reference) (OtherBodyIndex :type Integer) (bFromSweep :type Boolean) (SweepResult :type Hit%20Result%20Structure%20%28by%20ref%29))
  (bind _textentry (Variables|Default|GetTextEntry))
  (if (not (or (Utilities|Array|IsEmpty _textentry) (Variables|Default|GetHasTriggeredEntryText)))
    (CallFunction|NextDialogue OtherActor _textentry)
    (Variables|Default|SetHasTriggeredEntryText true)))

(event OnComponentEndOverlap(Box)
  (params (OverlappedComponent :type Primitive%20Component%20Object%20Reference) (OtherActor :type Actor%20Object%20Reference) (OtherComp :type Primitive%20Component%20Object%20Reference) (OtherBodyIndex :type Integer))
  (bind _textexit (Variables|Default|GetTextExit))
  (if (not (or (Variables|Default|GetHasTriggeredExitText) (Utilities|Array|IsEmpty _textexit)))
    (CallFunction|NextDialogue OtherActor _textexit)
    (Variables|Default|SetHasTriggeredExitText true)))

(event Custom|GoTo%20Talk
  (if (Utilities|Array|ContainsItem (Collision|GetOverlappingActors (Variables|Default|GetBox) "/Game/CouchGame2025/Blueprint/BP_Character.BP_Character_C" :!class /Script/Engine.PrimitiveComponent) (Variables|Default|GetChara))
    (Default|Talk self (Variables|Default|GetTextEntry))
    (else
      (Default|Talk self (Variables|Default|GetTextExit)))))

(event EventTalk
  (params (Text :type Array%20of%20Strings))
  (Math|Integer|IncrementInt (Variables|Default|GetTextIndex)
    (:%20%20
      (if (< (Variables|Default|GetTextIndex) (Utilities|Array|Length Text))
        (Development|PrintString (Utilities|Array|Get(acopy) Text (Variables|Default|GetTextIndex)))
        (Utilities|IsValid (Variables|Default|GetUI)
          (:Is%20Valid
            _)
          (:Is%20Not%20Valid
            (bind _returnvalue (UserInterface|CreateWidget "/Game/CouchGame2025/Widget/WBP_Dialogue.WBP_Dialogue_C" (Game|GetPlayerController 0)))
            (bind _output_get (Variables|Default|SetUI _returnvalue))
            (UserInterface|Viewport|AddtoViewport _output_get 0)))
        (Rendering|Components|TextRender|SetText (Variables|/Game/CouchGame2025/Widget/WBP_Dialogue.WBP_Dialogue_C|GetDialogueText _output_get) (Utilities|Text|ToText(String) (Utilities|Array|Get(acopy) Text (Variables|Default|GetTextIndex))))
        (else
          (Variables|Default|SetTextIndex -1)
          (Utilities|IsValid (Variables|Default|GetUI)
            (:Is%20Valid
              (Widget|RemovefromParent (Variables|Default|GetUI))
              (Variables|Default|SetUI 0))
            (:Is%20Not%20Valid
              _))
          (bind _outactors (Actor|GetAllActorsOfClass "/Game/CouchGame2025/Blueprint/BP_Character.BP_Character_C"))
          (for _array_element _outactors
            (EventDispatchers|UnbindallEventsfromOnNextDialogue _array_element)
            (bind _aspc_couch_game_2025 (Utilities|Casting|CastToPC_CouchGame2025 (Pawn|GetController _array_element)))
            (bind _returnvalue_2 (CallFunction|GetMappingContextfromDeviceId (Variables|/Game/CouchGame2025/Blueprint/BP_Character.BP_Character_C|GetInputId _array_element)))
            (Input|AddMappingContext (PlayerController|LocalPlayerSubsystems|GetEnhancedInputLocalPlayerSubsystem _aspc_couch_game_2025) _returnvalue_2 10 "(bIgnoreAllPressedKeysUntilRelease=True,bForceImmediately=False,bNotifyUserSettings=False)")
            (Input|RemoveMappingContext (PlayerController|LocalPlayerSubsystems|GetEnhancedInputLocalPlayerSubsystem _aspc_couch_game_2025) "/Game/CouchGame2025/Input/IMC_Dialogue.IMC_Dialogue" "(bIgnoreAllPressedKeysUntilRelease=True,bForceImmediately=False,bNotifyUserSettings=False)")))))))

(event EventBeginPlay
  (bind _datatable (Variables|Default|GetDataTable))
  (bind (_datatable_2 _rowname) (Utilities|Struct|BreakDataTableRowHandle _datatable))
  (bind _returnvalue (Utilities|GetDataTableRow _datatable_2 _rowname)
    (:then
      (bind _output_get (Variables|Default|SetDataTableRow _returnvalue))
      (Variables|Default|SetTextEntry (.EntryDialogueLines (Utilities|Struct|BreakS_DialogueRow _output_get)))
      (Variables|Default|SetTextExit (.ExitDialogueLines (Utilities|Struct|BreakS_DialogueRow _output_get)))
      (Development|PrintString (Utilities|String|Append "Data Row Loaded : " (.Name (Utilities|Struct|BreakS_DialogueRow _output_get))) true true "(R=0.000000,G=0.660000,B=1.000000,A=1.000000)" 5.0))
    (:RowNotFound
      (Development|PrintString (Utilities|String|Append "Row not found on : " (Utilities|GetObjectName self))))))

(fn ConstructionScript)

(fn NextDialogue
  (params (Chara :type Actor%20Object%20Reference) (Text :type Array%20of%20Strings))
  (if (< (Variables|Default|GetTextIndex) (Utilities|Array|Length Text))
    (bind _asbp_character (Utilities|Casting|CastToBP_Character Chara))
    (Variables|Default|SetChara _asbp_character)
    (EventDispatchers|BindEventtoOnNextDialogue _asbp_character (EventDispatchers|CreateEvent :!event Custom|GoTo%20Talk))
    (CallFunction|Talk Text)
    ;[0.15 0.15 0.15 0.5] Disable Player Inputs
    (bind _outactors (Actor|GetAllActorsOfClass "/Game/CouchGame2025/Blueprint/BP_Character.BP_Character_C"))
    (for _array_element _outactors
      (bind _aspc_couch_game_2025 (Utilities|Casting|CastToPC_CouchGame2025 (Pawn|GetController _array_element)))
      (bind _returnvalue (CallFunction|GetMappingContextfromDeviceId (Variables|/Game/CouchGame2025/Blueprint/BP_Character.BP_Character_C|GetInputId _array_element)))
      (Input|RemoveMappingContext (PlayerController|LocalPlayerSubsystems|GetEnhancedInputLocalPlayerSubsystem _aspc_couch_game_2025) _returnvalue "(bIgnoreAllPressedKeysUntilRelease=True,bForceImmediately=False,bNotifyUserSettings=False)")
      (Input|AddMappingContext (PlayerController|LocalPlayerSubsystems|GetEnhancedInputLocalPlayerSubsystem _aspc_couch_game_2025) "/Game/CouchGame2025/Input/IMC_Dialogue.IMC_Dialogue" 1000000000 "(bIgnoreAllPressedKeysUntilRelease=True,bForceImmediately=False,bNotifyUserSettings=False)"))))

(fn Talk2
  (params (NewParam :type Array%20of%20Strings))
  (bind _textindex (Variables|Default|GetTextIndex))
  (Math|Integer|IncrementInt _textindex
    (:%20%20
      (if (< _textindex (Utilities|Array|Length NewParam))
        (Development|PrintString (Utilities|Array|Get(acopy) NewParam (Variables|Default|GetTextIndex)))
        (Utilities|IsValid (Variables|Default|GetUI)
          (:Is%20Valid
            _)
          (:Is%20Not%20Valid
            (bind _returnvalue (UserInterface|CreateWidget "/Game/CouchGame2025/Widget/WBP_Dialogue.WBP_Dialogue_C" (Game|GetPlayerController 0)))
            (bind _output_get (Variables|Default|SetUI _returnvalue))
            (UserInterface|Viewport|AddtoViewport _output_get 0)))
        (Rendering|Components|TextRender|SetText (Variables|/Game/CouchGame2025/Widget/WBP_Dialogue.WBP_Dialogue_C|GetDialogueText _output_get) (Utilities|Text|ToText(String) (Utilities|Array|Get(acopy) NewParam (Variables|Default|GetTextIndex))))
        (else
          (Widget|RemovefromParent (Variables|Default|GetUI))
          (bind _outactors (Actor|GetAllActorsOfClass "/Game/CouchGame2025/Blueprint/BP_Character.BP_Character_C"))
          (for _array_element _outactors
            (EventDispatchers|UnbindallEventsfromOnNextDialogue _array_element)
            (bind _aspc_couch_game_2025 (Utilities|Casting|CastToPC_CouchGame2025 (Pawn|GetController _array_element)))
            (bind _returnvalue_2 (CallFunction|GetMappingContextfromDeviceId (Variables|/Game/CouchGame2025/Blueprint/BP_Character.BP_Character_C|GetInputId _array_element)))
            (Input|AddMappingContext (PlayerController|LocalPlayerSubsystems|GetEnhancedInputLocalPlayerSubsystem _aspc_couch_game_2025) _returnvalue_2 10 "(bIgnoreAllPressedKeysUntilRelease=True,bForceImmediately=False,bNotifyUserSettings=False)")))))))