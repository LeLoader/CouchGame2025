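; BP_Injector is a resource injector with a gauge that fills as its RessourceContainer updates, via a dynamic material's "hauteur" parameter.
; When full, or on CE_empty, it broadcasts OnContainerFull with SwitchSpeed and plays a reversed Timeline lasting according to SwitchSpeed.
; That Timeline drains the gauge, grows a sphere and moves the camera along a spline, aimed along a target spline.
; The sphere is hidden when it finishes.
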(event OnContainerFullBP(RessourceContainer)
  (bind _splinecamera (Variables|Default|GetSplineCamera))
  (Default|CallOnContainerFull (Variables|Default|GetSwitchSpeed))
  (bind _float (Timeline|Timeline ReverseFromEnd)
    (:Update
      (Rendering|Material|SetScalarParameterValue (Variables|Default|GetJauge%20Material) "hauteur" _float :!class /Script/Engine.MaterialInstanceDynamic)
      (Transformation|SetRelativeScale3D (Variables|Default|GetSphere) (Math|Vector|MakeVector (* (- 1.0 _float) (Variables|Default|GetMaxSize)) (* (- 1.0 _float) (Variables|Default|GetMaxSize)) (* (- 1.0 _float) (Variables|Default|GetMaxSize))))
      (Transformation|SetWorldLocationAndRotation (Variables|Default|GetCamera) (Spline|GetLocationatDistanceAlongSpline _splinecamera (Math|Float|Lerp 0.0 (Spline|GetSplineLength _splinecamera) (- 1.0 _float)) "World") (Math|Rotator|FindLookatRotation (Spline|GetLocationatDistanceAlongSpline _splinecamera (Math|Float|Lerp 0.0 (Spline|GetSplineLength _splinecamera) (- 1.0 _float)) "World") (Spline|GetLocationatDistanceAlongSpline (Variables|Default|GetSplineTargetPosition) (Math|Float|Lerp 0.0 (Spline|GetSplineLength (Variables|Default|GetSplineTargetPosition)) (- 1.0 _float)) "World")) false false))
    (:Finished
      (Rendering|SetVisibility (Variables|Default|GetSphere) false false))))

(event Custom|OnRessourceUpdated_Event
  (params (NewRessourceAmount :type Float%20%28single-precision%29) (OldRessourceAmount :type Float%20%28single-precision%29))
  (bind _jauge_material (Variables|Default|GetJauge%20Material))
  (bind _returnvalue (Rendering|Material|GetScalarParameterValue _jauge_material "hauteur" :!class /Script/Engine.MaterialInstanceDynamic))
  (Rendering|Material|SetScalarParameterValue _jauge_material "hauteur" (Math|Float|Clamp(Float) (+ _returnvalue (/ (/ NewRessourceAmount (Variables|/Script/CouchGame2025.RessourceContainerComponent|GetMaxRessourceAmount (Variables|Default|GetRessourceContainer))) 2.0))) :!class /Script/Engine.MaterialInstanceDynamic))

(event Custom|CE_empty
  (bind _splinecamera (Variables|Default|GetSplineCamera))
  (Default|CallOnContainerFull (Variables|Default|GetSwitchSpeed))
  (bind _float (Timeline|Timeline ReverseFromEnd)
    (:Update
      (Rendering|Material|SetScalarParameterValue (Variables|Default|GetJauge%20Material) "hauteur" _float :!class /Script/Engine.MaterialInstanceDynamic)
      (Transformation|SetRelativeScale3D (Variables|Default|GetSphere) (Math|Vector|MakeVector (* (- 1.0 _float) (Variables|Default|GetMaxSize)) (* (- 1.0 _float) (Variables|Default|GetMaxSize)) (* (- 1.0 _float) (Variables|Default|GetMaxSize))))
      (Transformation|SetWorldLocationAndRotation (Variables|Default|GetCamera) (Spline|GetLocationatDistanceAlongSpline _splinecamera (Math|Float|Lerp 0.0 (Spline|GetSplineLength _splinecamera) (- 1.0 _float)) "World") (Math|Rotator|FindLookatRotation (Spline|GetLocationatDistanceAlongSpline _splinecamera (Math|Float|Lerp 0.0 (Spline|GetSplineLength _splinecamera) (- 1.0 _float)) "World") (Spline|GetLocationatDistanceAlongSpline (Variables|Default|GetSplineTargetPosition) (Math|Float|Lerp 0.0 (Spline|GetSplineLength (Variables|Default|GetSplineTargetPosition)) (- 1.0 _float)) "World")) false false))
    (:Finished
      (Rendering|SetVisibility (Variables|Default|GetSphere) false false))))

(event EventBeginPlay
  (EventDispatchers|AssignOnRessourceUpdated (Variables|Default|GetRessourceContainer) (EventDispatchers|CreateEvent :!event Custom|OnRessourceUpdated_Event))
  (bind _returnvalue (Rendering|Material|CreateDynamicMaterialInstance "/Game/CouchGame2025/Asset/jauge/MI_jauge_injecteur.MI_jauge_injecteur" "None" "None" :!class /Script/Engine.KismetMaterialLibrary))
  (bind _output_get (Variables|Default|SetJauge%20Material _returnvalue))
  (Rendering|Material|SetMaterial (Variables|Default|GetMeshComponent) 1 _output_get)
  (Components|Timeline|SetPlayRate (Variables|Default|GetTimeline) (/ 1.0 (Variables|Default|GetSwitchSpeed))))

(fn ConstructionScript)