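; BP_Flamethrower is a usable flamethrower that shows its Niagara effect only while in use.
; StartUse and StopUse call their parent versions, then activate or deactivate the Niagara component.
; BeginPlay sets the effect active and immediately deactivates it, so it starts off.
; Tick is empty, and a node matching actor rotation to player 0's control rotation is left unconnected.
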(event EventBeginPlay
  (bind _niagara (Variables|Default|GetNiagara))
  (Components|Activation|SetActive _niagara true false)
  (Components|Activation|Deactivate _niagara))

(event EventStartUse
  (|CallParentFunction)
  (Components|Activation|Activate (Variables|Default|GetNiagara) false))

(event EventStopUse
  (|CallParentFunction)
  (Components|Activation|Deactivate (Variables|Default|GetNiagara)))

(event EventTick
  (params (DeltaSeconds :type Float%20%28single-precision%29)))

(fn ConstructionScript)