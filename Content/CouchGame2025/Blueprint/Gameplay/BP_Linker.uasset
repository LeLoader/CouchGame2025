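; BP_Linker is an actor that joins an external and an internal transfer point along a spline.
; On BeginPlay it casts each child actor to BP_TransfertPoint and sets the opposite point as its linked actor.
; Both points also receive the same Spline component, so the link works as a two-way pair sharing one path.
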(event EventBeginPlay
  (bind _spline (Variables|Default|GetSpline))
  (bind _asbp_transfert_point (Utilities|Casting|CastToBP_TransfertPoint (Variables|/Script/Engine.ChildActorComponent|GetChildActor (Variables|Default|GetExternalTransfertPoint))))
  (Class|TransfertPoint|SetLinkedActor _asbp_transfert_point (Variables|/Script/Engine.ChildActorComponent|GetChildActor (Variables|Default|GetInternalTransfertPoint)))
  (Class|TransfertPoint|SetSplineComponent _asbp_transfert_point _spline)
  (bind _asbp_transfert_point_2 (Utilities|Casting|CastToBP_TransfertPoint (Variables|/Script/Engine.ChildActorComponent|GetChildActor (Variables|Default|GetInternalTransfertPoint))))
  (Class|TransfertPoint|SetLinkedActor _asbp_transfert_point_2 (Variables|/Script/Engine.ChildActorComponent|GetChildActor (Variables|Default|GetExternalTransfertPoint)))
  (Class|TransfertPoint|SetSplineComponent _asbp_transfert_point_2 _spline))

(fn ConstructionScript)