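; BP_WidgetWrapper is an actor that hosts a WBP_InteractButton widget and animates it appearing and disappearing.
; On BeginPlay it caches the widget, resets its material to zero and scales the timeline rate by TotalTransitionTime.
; Show plays the timeline, feeding Alpha into the widget's UpdateMaterial, and Hide reverses it.
; When the reverse finishes, the actor detaches itself from whatever it was attached to.
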(event Custom|Show
  (bind (_direction _alpha) (Timeline|Timeline Play)
    (:Update
      (Default|UpdateMaterial (Variables|Default|GetWidgetBP) _alpha))
    (:Finished
      (if (Utilities|Enum|Equal(Enum) _direction "Backward")
        (Transformation|DetachFromActor "KeepRelative" "KeepRelative" "KeepRelative")))))

(event Custom|Hide
  (bind (_direction _alpha) (Timeline|Timeline Reverse)
    (:Update
      (Default|UpdateMaterial (Variables|Default|GetWidgetBP) _alpha))
    (:Finished
      (if (Utilities|Enum|Equal(Enum) _direction "Backward")
        (Transformation|DetachFromActor "KeepRelative" "KeepRelative" "KeepRelative")))))

(event EventBeginPlay
  (bind _widget (Variables|Default|GetWidget))
  (bind _returnvalue (UserInterface|GetWidget _widget))
  (Variables|/Script/UMG.Widget|SetVisibility _returnvalue "Visible")
  (bind _aswbp_interact_button (Utilities|Casting|CastToWBP_InteractButton _returnvalue))
  (Variables|Default|SetWidgetBP _aswbp_interact_button)
  (Components|Timeline|SetPlayRate (Variables|Default|GetTimeline) (/ 1.0 (Variables|Default|GetTotalTransitionTime)))
  (Default|UpdateMaterial _aswbp_interact_button 0.0))

(fn ConstructionScript)