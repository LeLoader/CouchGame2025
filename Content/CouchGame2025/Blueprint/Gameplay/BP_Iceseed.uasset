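; BP_Iceseed is a meltable ice block that makes nearby characters slide and shows them a frozen-screen effect.
; Overlap volumes lower and restore character friction and toggle that effect.
; IceContainer events drive the melting Niagara effect and block material, and burning plays a melt sound.
; When the container empties, the block and volumes switch off, the mesh starts blocking a trace channel, and Tick fades the verglas decal out.
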(event OnComponentBeginOverlap(Box)
  (params (OverlappedComponent :type Primitive%20Component%20Object%20Reference) (OtherActor :type Actor%20Object%20Reference) (OtherComp :type Primitive%20Component%20Object%20Reference) (OtherBodyIndex :type Integer) (bFromSweep :type Boolean) (SweepResult :type Hit%20Result%20Structure%20%28by%20ref%29))
  (bind _asbp_character (Utilities|Casting|CastToBP_Character OtherActor))
  (Variables|/Script/Engine.CharacterMovementComponent|SetBrakingFriction (Variables|/Script/Engine.Character|GetCharacterMovement _asbp_character) 0.1)
  (Variables|/Script/Engine.CharacterMovementComponent|SetBrakingDecelerationWalking (Variables|/Script/Engine.Character|GetCharacterMovement _asbp_character) 3e+02)
  (Variables|/Script/Engine.CharacterMovementComponent|SetGroundFriction (Variables|/Script/Engine.Character|GetCharacterMovement _asbp_character) 0.1))

(event OnComponentEndOverlap(Box)
  (params (OverlappedComponent :type Primitive%20Component%20Object%20Reference) (OtherActor :type Actor%20Object%20Reference) (OtherComp :type Primitive%20Component%20Object%20Reference) (OtherBodyIndex :type Integer))
  (bind _asbp_character (Utilities|Casting|CastToBP_Character OtherActor))
  (Variables|/Script/Engine.CharacterMovementComponent|SetBrakingFriction (Variables|/Script/Engine.Character|GetCharacterMovement _asbp_character) 2.0)
  (Variables|/Script/Engine.CharacterMovementComponent|SetBrakingDecelerationWalking (Variables|/Script/Engine.Character|GetCharacterMovement _asbp_character) 2e+03)
  (Variables|/Script/Engine.CharacterMovementComponent|SetGroundFriction (Variables|/Script/Engine.Character|GetCharacterMovement _asbp_character) 8.0))

(event OnComponentBeginOverlap(FrozenScreen)
  (params (OverlappedComponent :type Primitive%20Component%20Object%20Reference) (OtherActor :type Actor%20Object%20Reference) (OtherComp :type Primitive%20Component%20Object%20Reference) (OtherBodyIndex :type Integer) (bFromSweep :type Boolean) (SweepResult :type Hit%20Result%20Structure%20%28by%20ref%29))
  (bind _asbp_character (Utilities|Casting|CastToBP_Character OtherActor))
  (Default|ShowFrozenCamera _asbp_character))

(event OnComponentEndOverlap(FrozenScreen)
  (params (OverlappedComponent :type Primitive%20Component%20Object%20Reference) (OtherActor :type Actor%20Object%20Reference) (OtherComp :type Primitive%20Component%20Object%20Reference) (OtherBodyIndex :type Integer))
  (bind _asbp_character (Utilities|Casting|CastToBP_Character OtherActor))
  (Default|HideCompletly _asbp_character))

(event Custom|OnContainerEmpty
  (bind _bigiceblock (Variables|Default|GetBigIceBlock))
  (Variables|Default|SetTargetOpacity 0.0)
  (Components|Activation|Deactivate (Variables|Default|GetNiagara))
  (Rendering|SetVisibility _bigiceblock false false)
  (Collision|SetCollisionEnabled _bigiceblock "NoCollision")
  (Collision|SetCollisionResponsetoChannel (Variables|Character|GetMesh) "ECC_GameTraceChannel2" "ECR_Block")
  (Collision|SetCollisionEnabled (Variables|Default|GetBox) "NoCollision")
  (Collision|SetCollisionEnabled (Variables|Default|GetFrozenScreen) "NoCollision"))

(event Custom|OnRessourceUpdated
  (params (NewRessourceAmount :type Float%20%28single-precision%29) (OldRessourceAmount :type Float%20%28single-precision%29))
  (Components|Activation|Activate (Variables|Default|GetNiagara) false)
  (Rendering|Material|SetScalarParameterValueonMaterials (Variables|Default|GetBigIceBlock) "Alive > Frozen" (- 1.0 (/ NewRessourceAmount (Variables|/Script/CouchGame2025.RessourceContainerComponent|GetMaxRessourceAmount (Variables|Default|GetIceContainer))))))

(event Custom|OnRessourceStartMoving
  (Components|Activation|Activate (Variables|Default|GetNiagara) true))

(event Custom|OnRessourceStopMoving
  (Components|Activation|Deactivate (Variables|Default|GetNiagara)))

(event Custom|OnDestroyed_Event
  (params (DestroyedActor :type Actor%20Object%20Reference)))

(event EventBeginPlay
  (bind _icecontainer (Variables|Default|GetIceContainer))
  (bind _returnvalue (Rendering|Material|CreateDynamicMaterialInstance "/Game/CouchGame2025/Asset/verglas/MA_verglas.MA_verglas" "None" "None" :!class /Script/Engine.KismetMaterialLibrary))
  (bind _output_get (Variables|Default|SetDynamicDecalMaterial _returnvalue))
  (Rendering|Components|Decal|SetDecalMaterial (Variables|Default|GetDecal) _output_get)
  (EventDispatchers|AssignOnRessourceUpdated _icecontainer (EventDispatchers|CreateEvent :!event Custom|OnRessourceUpdated))
  (EventDispatchers|AssignOnContainerEmptyBP _icecontainer (EventDispatchers|CreateEvent :!event Custom|OnContainerEmpty))
  (bind _output_get_2 (Variables|Default|SetTargetOpacity (Variables|Default|GetCurrentOpacity)))
  (Rendering|Material|SetScalarParameterValue (Variables|Default|GetDynamicDecalMaterial) "opacity" _output_get_2 :!class /Script/Engine.MaterialInstanceDynamic)
  (Game|AssignOnDestroyed (delegate Custom|OnDestroyed_Event)))

(event EventTick
  (params (DeltaSeconds :type Float%20%28single-precision%29))
  (bind _output_get (Variables|Default|SetCurrentOpacity (Math|Interpolation|FInterptoConstant (Variables|Default|GetCurrentOpacity) (Variables|Default|GetTargetOpacity) DeltaSeconds (Variables|Default|GetIceMeltingSpeed))))
  (Rendering|Material|SetScalarParameterValue (Variables|Default|GetDynamicDecalMaterial) "opacity" _output_get :!class /Script/Engine.MaterialInstanceDynamic))

(event EventOnBurnStarted
  (bind _returnvalue (Audio|CreateSound2D "/Game/CouchGame2025/Audio/MetaSound/MS_IceHeart_Melt.MS_IceHeart_Melt" 1.0 1.0 0.0 0))
  (Audio|Components|Audio|Play _returnvalue 0.0)
  (Development|PrintString "Hello"))

(fn ConstructionScript)

(fn GetMaxWater
  (return (Variables|/Script/CouchGame2025.RessourceContainerComponent|GetMaxRessourceAmount (Variables|Default|GetWaterContainer))))