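; BP_Region is a region actor that tracks waste, injector and ice seed objectives and broadcasts their progress and the region's completion.
; BeginPlay builds objective objects from a data table and binds their events.
; Tag-matched trash destruction and ice seed events feed progress, but the binding switch is fixed to WASTE and the injector branch is unfinished.
; The completion check returns true even when it finds an incomplete objective.
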(event Custom|OnTrashDestroyed
  (params (Trash :type Actor%20Object%20Reference))
  (if (Actor|ActorHasTag Trash (Variables|Default|GetTag))
    (Default|ProgressObjective (CallFunction|GetObjectivefromObjectiveType "NewEnumerator0") 1.0 "NewEnumerator0")))

(event Custom|OnIceUnfreezed
  (Default|ProgressObjective (CallFunction|GetObjectivefromObjectiveType "NewEnumerator2") 1.0 "NewEnumerator0"))

(event Custom|OnObjectiveCompleted
  (params (Type :type E_ObjectiveType%20Enum :default "NewEnumerator0"))
  (if (CallFunction|IsRegionCompleted)
    ;[0.15 0 0 0.5] Unlock next region, prob from gm
    (Default|CallOnRegionCompleted)))

(event Custom|OnObjectiveProgresseddd
  (params (NewProgression :type Float%20%28double-precision%29) (Type :type E_ObjectiveType%20Enum :default "NewEnumerator0"))
  (Default|CallOnObjectiveProgressed NewProgression Type (Variables|Default|GetTag)))

(event EventBeginPlay
  (bind _outrownames (DataTable|GetDataTableRowNames (Variables|Default|GetObjectivesDataTable)))
  (for _array_element _outrownames
    (bind _returnvalue (Utilities|GetDataTableRow (Variables|Default|GetObjectivesDataTable) _array_element)
      (:then
        (bind _returnvalue_2 (Game|ConstructObjectfromClass (CallFunction|GetObjectiveClassfromObjectiveType (.Type (Utilities|Struct|BreakS_Objective _returnvalue))) (.Goal (Utilities|Struct|BreakS_Objective _returnvalue))))
        (Utilities|Array|Add (Variables|Default|GetObjectives) _returnvalue_2)
        (EventDispatchers|AssignOnObjectiveCompleted _returnvalue_2 (EventDispatchers|CreateEvent :!event Custom|OnObjectiveCompleted))
        (EventDispatchers|AssignOnObjectiveProgressed _returnvalue_2 (EventDispatchers|CreateEvent :!event Custom|OnObjectiveProgresseddd))
        (switch Utilities|FlowControl|Switch|SwitchonE_ObjectiveType "NewEnumerator0"
          (:NewEnumerator0
            (bind _returnvalue_3 (Actor|GetActorOfClass "/Game/CouchGame2025/Blueprint/BP_BlackHole.BP_BlackHole_C"))
            (EventDispatchers|BindEventtoOnTrashDestroyed _returnvalue_3 (EventDispatchers|CreateEvent :!event Custom|OnTrashDestroyed)))
          (:NewEnumerator1
            (Actor|GetAllActorsOfClass 0))
          (:NewEnumerator2
            (bind _outactors (Actor|GetAllActorsOfClass "/Game/CouchGame2025/Blueprint/Gameplay/BP_Iceseed.BP_Iceseed_C"))
            (for _array_element_2 _outactors
              (if (Actor|ActorHasTag _array_element_2 (Variables|Default|GetTag))
                (EventDispatchers|AssignOnIceSeedPickable _array_element_2 (EventDispatchers|CreateEvent :!event Custom|OnIceUnfreezed))))))))))

(fn ConstructionScript)

(fn IsRegionCompleted
  (bind _array_element (Utilities|Array|ForEachLoopwithBreak (Variables|Default|GetObjectives) :!label _label)
    (:LoopBody
      (if (not (Variables|/Game/CouchGame2025/Data/Objectives/Objective.Objective_C|GetbIsCompleted _array_element))
        (goto _label Break)))
    (:Completed
      (return true))))

(fn GetObjectiveClassfromObjectiveType
  (params (ObjectiveType :type E_ObjectiveType%20Enum :default "NewEnumerator0"))
  (return (Utilities|Select :Index ObjectiveType :NewEnumerator0 "/Game/CouchGame2025/Data/Objectives/TrashObjective.TrashObjective_C" :NewEnumerator1 "/Game/CouchGame2025/Data/Objectives/InjectorObjective.InjectorObjective_C" :NewEnumerator2 "/Game/CouchGame2025/Data/Objectives/IceseedObjective.IceseedObjective_C")))

(fn GetObjectivefromObjectiveType
  (params (Type :type E_ObjectiveType%20Enum :default "NewEnumerator0"))
  (for _array_element (Variables|Default|GetObjectives)
    (if (Utilities|Enum|Equal(Enum) (Variables|/Game/CouchGame2025/Data/Objectives/Objective.Objective_C|GetType _array_element) Type)
      (return _array_element)))
  (return 0))