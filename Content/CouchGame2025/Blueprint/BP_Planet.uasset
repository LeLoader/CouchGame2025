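; BP_Planet is a planet actor that switches the gravity mode of the BP_Andro character.
; It caches the first BP_Andro found at BeginPlay.
; Entering the InternalPlanet volume turns off UseExternalGravityDirection on the character's PlanetaryMovementComponent, leaving turns it on, and both call UpdateGravity.
; The overlap handlers never check the overlapping actor, so any overlap affects that cached character.
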(event OnComponentBeginOverlap(InternalPlanet)
  (params (OverlappedComponent :type Primitive%20Component%20Object%20Reference) (OtherActor :type Actor%20Object%20Reference) (OtherComp :type Primitive%20Component%20Object%20Reference) (OtherBodyIndex :type Integer) (bFromSweep :type Boolean) (SweepResult :type Hit%20Result%20Structure%20%28by%20ref%29))
  (bind _character (Variables|Default|GetCharacter))
  (Variables|/Script/CouchGame2025.PlanetaryMovementComponent|SetUseExternalGravityDirection (Variables|/Game/ThirdPerson/Blueprints/BP_Andro.BP_Andro_C|GetPlanetary%20Movement%20Component _character) false)
  (Default|UpdateGravity _character))

(event OnComponentEndOverlap(InternalPlanet)
  (params (OverlappedComponent :type Primitive%20Component%20Object%20Reference) (OtherActor :type Actor%20Object%20Reference) (OtherComp :type Primitive%20Component%20Object%20Reference) (OtherBodyIndex :type Integer))
  (bind _character (Variables|Default|GetCharacter))
  (Variables|/Script/CouchGame2025.PlanetaryMovementComponent|SetUseExternalGravityDirection (Variables|/Game/ThirdPerson/Blueprints/BP_Andro.BP_Andro_C|GetPlanetary%20Movement%20Component _character) true)
  (Default|UpdateGravity _character))

(event EventBeginPlay
  (bind _returnvalue (Actor|GetActorOfClass "/Game/ThirdPerson/Blueprints/BP_Andro.BP_Andro_C"))
  (Variables|Default|SetCharacter _returnvalue))

(fn ConstructionScript)