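; Player character for a planetary-gravity game with a two-player rope constraint, using PlanetaryMovementComponent for gravity.
; PickupComponent target changes attach or hide a spawned interaction widget, while WaterTank updates drive the tank gauge material.
; MoveAlongSpline uses a Timeline to carry the character along a spline either way, inverting it via a timeline event.
; Inputs handle rope toggle and partner teleport, jump Niagara, and shortcuts for switching sides, returning to PlayerStart and completing Region1.
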(event Custom|OnNewInteractionTarget
  (params (NewInteractionTarget :type Actor%20Object%20Reference) (OldInteractionTarget :type Actor%20Object%20Reference))
  (bind _widgetwrapper (Variables|Default|GetWidgetWrapper))
  (bind _widget (Variables|/Game/CouchGame2025/Blueprint/Gameplay/BP_WidgetWrapper.BP_WidgetWrapper_C|GetWidget _widgetwrapper))
  (bind _returnvalue (UserInterface|GetWidget _widget))
  (if (Utilities|IsValid NewInteractionTarget)
    (Widget|SetVisibility _returnvalue "Visible")
    (Transformation|AttachActorToActor _widgetwrapper NewInteractionTarget "None" "SnapToTarget" "SnapToTarget" "SnapToTarget" false)
    (else
      (Widget|SetVisibility _returnvalue "Hidden")
      (Transformation|DetachFromActor _widgetwrapper "KeepWorld" "KeepWorld" "KeepWorld"))))

(event Custom|OnWaterTankUpdated
  (params (NewRessourceAmount :type Float%20%28single-precision%29) (OldRessourceAmount :type Float%20%28single-precision%29))
  (Rendering|Material|SetScalarParameterValueonMaterials (Variables|Default|GetSM_WaterTank) "hauteur" NewRessourceAmount))

(event Input|EnhancedActionEvents|EnhancedInputActionIA_Rope
  (params (ActionValue :type Float%20%28double-precision%29) (ElapsedSeconds :type Float%20%28double-precision%29) (TriggeredSeconds :type Float%20%28double-precision%29) (InputAction :type Input%20Action%20Object%20Reference :default "/Game/CouchGame2025/Input/Inputs/IA_Rope.IA_Rope"))
  (:Canceled
    (bind _returnvalue (Actor|GetActorOfClass "/Game/CouchGame2025/Blueprint/BP_PlayerConstraint.BP_PlayerConstraint_C" :!label _label))
    (Default|Toggle _returnvalue))
  (:Completed
    (bind _returnvalue_2 (Actor|GetActorOfClass "/Game/CouchGame2025/Blueprint/BP_PlayerConstraint.BP_PlayerConstraint_C"))
    (Default|TeleporttoOtherPlayer _returnvalue_2 self)
    (goto _label)))

(event Input|EnhancedActionEvents|EnhancedInputActionIA_TeleportToOtherSide
  (params (ActionValue :type Boolean) (ElapsedSeconds :type Float%20%28double-precision%29) (TriggeredSeconds :type Float%20%28double-precision%29) (InputAction :type Input%20Action%20Object%20Reference :default "/Game/CouchGame2025/Input/Inputs/IA_TeleportToOtherSide.IA_TeleportToOtherSide"))
  (bind _returnvalue (Transformation|GetActorUpVector))
  (:Started
    (bind (_outhit _returnvalue_2) (Collision|LineTraceByChannel (+ (Transformation|GetActorLocation) (* _returnvalue 1e+03 -1.0)) (Transformation|GetActorLocation) "TraceTypeQuery1" false 0 "None"))
    (if _returnvalue_2
      (Transformation|SetActorLocation (+ (.ImpactPoint (Collision|BreakHitResult _outhit)) (* _returnvalue 5e+01 -1.0)) false true))))

(event Input|EnhancedActionEvents|EnhancedInputActionIA_Jump
  (params (ActionValue :type Boolean) (ElapsedSeconds :type Float%20%28double-precision%29) (TriggeredSeconds :type Float%20%28double-precision%29) (InputAction :type Input%20Action%20Object%20Reference :default "/Game/CouchGame2025/Input/Inputs/IA_Jump.IA_Jump"))
  (:Started
    (Components|Activation|Activate (Variables|Default|GetNiagara) true)))

(event Input|EnhancedActionEvents|EnhancedInputActionIA_CompeteRegion1
  (params (ActionValue :type Boolean) (ElapsedSeconds :type Float%20%28double-precision%29) (TriggeredSeconds :type Float%20%28double-precision%29) (InputAction :type Input%20Action%20Object%20Reference :default "/Game/CouchGame2025/Input/Inputs/IA_CompeteRegion1.IA_CompeteRegion1"))
  (bind _outactors (Actor|GetAllActorsOfClasswithTag "/Game/CouchGame2025/Blueprint/Gameplay/BP_MeteorBase1.BP_MeteorBase1_C" "Region1"))
  (for _array_element _outactors
    (Transformation|Teleport _array_element "0, 0, 0" "0, 0, 0"))
  (bind _outactors_2 (Actor|GetAllActorsOfClasswithTag "/Game/CouchGame2025/Blueprint/Gameplay/BP_MeteorBase2.BP_MeteorBase2_C" "Region1"))
  (for _array_element_2 _outactors_2
    (Transformation|Teleport _array_element_2 "0, 0, 0" "0, 0, 0"))
  (bind _outactors_3 (Actor|GetAllActorsOfClasswithTag "/Script/CouchGame2025.IceSeed" "Region1"))
  (for _array_element_3 _outactors_3
    (Class|RessourceContainerComponent|RemoveRessource (Variables|/Script/CouchGame2025.IceSeed|GetIceContainer _array_element_3) (Variables|/Script/CouchGame2025.RessourceContainerComponent|GetCurrentRessourceAmount (Variables|/Script/CouchGame2025.IceSeed|GetIceContainer _array_element_3)))
    (Transformation|Teleport _array_element_3 "0, 0, 0" "0, 0, 0"))
  (bind _outactors_4 (Actor|GetAllActorsOfClasswithTag "/Game/CouchGame2025/Blueprint/Gameplay/NeededOnScene/BP_Region.BP_Region_C" "Region1"))
  (Class|RessourceContainerComponent|AddRessource (Variables|/Script/CouchGame2025.RessourceInjector|GetRessourceContainer (Variables|/Game/CouchGame2025/Blueprint/Gameplay/NeededOnScene/BP_Region.BP_Region_C|GetInjector (Utilities|Array|Get(acopy) _outactors_4))) (Variables|/Script/CouchGame2025.RessourceContainerComponent|GetMaxRessourceAmount (Variables|/Script/CouchGame2025.RessourceInjector|GetRessourceContainer (Variables|/Game/CouchGame2025/Blueprint/Gameplay/NeededOnScene/BP_Region.BP_Region_C|GetInjector (Utilities|Array|Get(acopy) _outactors_4))))))

(event Input|EnhancedActionEvents|EnhancedInputActionIA_TpToPS
  (params (ActionValue :type Boolean) (ElapsedSeconds :type Float%20%28double-precision%29) (TriggeredSeconds :type Float%20%28double-precision%29) (InputAction :type Input%20Action%20Object%20Reference :default "/Game/CouchGame2025/Input/Inputs/IA_TpToPS.IA_TpToPS"))
  (:Started
    (bind _returnvalue (Actor|GetActorOfClass "/Script/Engine.PlayerStart"))
    (Transformation|Teleport (Transformation|GetActorLocation _returnvalue) "0, 0, 0")))

(event EventBeginPlay
  (Input|AddMappingContext (PlayerController|LocalPlayerSubsystems|GetEnhancedInputLocalPlayerSubsystem (Game|GetPlayerController 0)) "/Game/CouchGame2025/Input/IMC_Debug.IMC_Debug" 0 "(bIgnoreAllPressedKeysUntilRelease=True,bForceImmediately=False,bNotifyUserSettings=False)")
  (CallFunction|UpdateGravity)
  (EventDispatchers|AssignOnNewInteractionTarget (Variables|Default|GetPickupComponent) (EventDispatchers|CreateEvent :!event Custom|OnNewInteractionTarget))
  (bind _returnvalue (Game|SpawnActorfromClass "/Game/CouchGame2025/Blueprint/Gameplay/BP_WidgetWrapper.BP_WidgetWrapper_C" (Math|Transform|MakeTransform "0, 0, 0" "0, 0, 0" "1.000000,1.000000,1.000000") "AlwaysSpawn" "MultiplyWithRoot" 0 0))
  (Variables|Default|SetWidgetWrapper _returnvalue)
  (EventDispatchers|AssignOnRessourceUpdated (Variables|Default|GetWaterTank) (delegate Custom|OnWaterTankUpdated))
  (bind _returnvalue_2 (Rendering|Material|CreateDynamicMaterialInstance (Variables|Default|GetSM_WaterTank) 1 "/Game/CouchGame2025/Asset/jauge/MA_jauge_Inst.MA_jauge_Inst" "None" :!class /Script/Engine.PrimitiveComponent))
  (Variables|Default|SetWaterTankMaterial _returnvalue_2)
  (Rendering|Material|SetScalarParameterValueonMaterials (Variables|Default|GetSM_WaterTank) "hauteur" 0.0))

(event EventMoveAlongSpline
  (params (Spline :type Spline%20Component%20Object%20Reference) (IsMovingForward :type Boolean))
  (Development|PrintString (Utilities|String|Append (Utilities|GetDisplayName self) " Started") true true "(R=1.000000,G=0.000000,B=0.000000,A=1.000000)" 2.0 "1")
  (Variables|Default|SetbIsWaiting true)
  (if IsMovingForward
    (bind _float (Timeline|Timeline PlayFromStart)
      (:Update
        (Transformation|SetActorLocationAndRotation (.location (Spline|GetTransformatDistanceAlongSpline Spline (Math|Float|Lerp 0.0 (Spline|GetSplineLength Spline) _float) "World" false)) (.rotation (Spline|GetTransformatDistanceAlongSpline Spline (Math|Float|Lerp 0.0 (Spline|GetSplineLength Spline) _float) "World" false))))
      (:Finished
        (Variables|Default|SetbIsWaiting false)
        (Development|PrintString (Utilities|String|Append (Utilities|GetDisplayName self) " Finished") true true "(R=1.000000,G=0.000000,B=0.000000,A=1.000000)" 2.0 "1")
        (Class|CouchGame2025Character|CallEventEndMovingAlongSpline))
      (:Event
        (Class|CouchGame2025Character|InvertCharacter)))
    (else
      (Timeline|Timeline ReverseFromEnd))))

(fn ConstructionScript)

(fn ExternalGravity
  (bind _planetary_movement_component (Variables|Default|GetPlanetary%20Movement%20Component))
  (Class|PlanetaryMovementComponent|UpdateGravityDirection _planetary_movement_component (Variables|/Script/CouchGame2025.PlanetaryMovementComponent|GetPlanetCenter _planetary_movement_component)))

(fn InvertGravity
  (Class|PlanetaryMovementComponent|InvertGravity (Variables|Default|GetPlanetary%20Movement%20Component)))

(fn UpdateGravity
  (Variables|Default|GetPlanetary%20Movement%20Component
    (:then)
    (:else
      (bind _asplanetary_movement_component (Utilities|Casting|CastToPlanetaryMovementComponent (Variables|Character|GetCharacterMovement)))
      (Variables|Default|SetPlanetary%20Movement%20Component _asplanetary_movement_component))))