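; Game mode for CouchGame2025 that drives the local multiplayer flow from start menu through character selection to gameplay.
; BeginPlay sets the Menu input mapping, views the tagged start camera and shows the start widget.
; StartSelection optionally blends to the selection camera, with a matching timer delaying the toggleable selection widget.
; StartGame adds the objective HUD, plays get-up animations on "Hide"-tagged skeletal mesh actors, then destroys them after a short delay.
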(event Custom|StartSelection
  (bind _pick_a (Variables|Default|GetPick%20A))
  (bind _returnvalue (Math|Float|SelectFloat 5.0 0.0 _pick_a))
  (bind _outactors (Actor|GetAllActorsOfClasswithTag "/Script/Engine.CameraActor" "SelectionCamera"))
  (Game|Player|SetViewTargetwithBlend (Game|GetPlayerController 0) (Utilities|Array|Get(acopy) _outactors) _returnvalue "VTBlend_EaseInOut" 3.0 false)
  (Utilities|Time|SetTimerbyEvent (delegate Custom|ShowSelection) _returnvalue))

(event Custom|ToggleCharacterSelectionWidget
  (bind _characterselectionwidget (Variables|Default|GetCharacterSelectionWidget))
  (if (UserInterface|Viewport|IsinViewport (Variables|Default|GetCharacterSelectionWidget))
    (Widget|RemovefromParent _characterselectionwidget)
    (else
      (UserInterface|Viewport|AddtoViewport _characterselectionwidget 0))))

(event Custom|StartGame
  (bind _returnvalue (UserInterface|CreateWidget "/Game/CouchGame2025/Widget/Objectives/WBP_CommonObjectiveHUD.WBP_CommonObjectiveHUD_C"))
  (bind _output_get (Variables|Default|SetObjectiveHUD _returnvalue))
  (UserInterface|Viewport|AddtoViewport _output_get 0)
  (bind _outactors (Actor|GetAllActorsOfClasswithTag "/Script/Engine.SkeletalMeshActor" "Hide"))
  (for _array_element _outactors
    (Components|Animation|PlayAnimation (Variables|/Script/Engine.SkeletalMeshActor|GetSkeletalMeshComponent _array_element) "/Game/CouchGame2025/Asset/animation/ANIM_Chara_getup_banch.ANIM_Chara_getup_banch" false))
  (Utilities|FlowControl|Delay 1.0)
  (bind _outactors_2 (Actor|GetAllActorsOfClasswithTag "/Script/Engine.SkeletalMeshActor" "Hide"))
  (for _array_element_2 _outactors_2
    (Actor|DestroyActor _array_element_2)))

(event Custom|ShowSelection
  (bind _returnvalue (UserInterface|CreateWidget "/Game/CouchGame2025/Widget/WBP_CharacterSelection.WBP_CharacterSelection_C" (Game|GetPlayerController 0)))
  (bind _output_get (Variables|Default|SetCharacterSelectionWidget _returnvalue))
  (UserInterface|Viewport|AddtoViewport _output_get 0))

(event EventBeginPlay
  (Class|LocalMultiplayerSubsystem|SetCurrentMappingType (Subsystems|GetLocalMultiplayerSubsystem) "Menu")
  (bind _outactors (Actor|GetAllActorsOfClasswithTag "/Script/Engine.CameraActor" "StartCamera"))
  (Game|Player|SetViewTargetwithBlend (Game|GetPlayerController 0) (Utilities|Array|Get(acopy) _outactors) 0.0 "VTBlend_Linear" 0.0 false)
  (bind _returnvalue (UserInterface|CreateWidget "/Game/CouchGame2025/Widget/WBP_Start.WBP_Start_C" (Game|GetPlayerController 0)))
  (UserInterface|Viewport|AddtoViewport _returnvalue 0))

(fn ConstructionScript)