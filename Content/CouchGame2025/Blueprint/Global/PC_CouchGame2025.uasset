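; Player controller for the local multiplayer couch game that routes each player's menu input to the shared character selection screen.
; BeginPlay caches the game mode and local multiplayer settings and finds the controller's own player index.
; Menu select input passes that index and the action value to the game mode's selection widget, throttled by a DoOnce that a timer resets.
; Debug events print the controlled pawn and connected users and input devices.
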(event Custom|CE_pawn
  (Development|PrintString (Utilities|GetDisplayName (Pawn|GetControlledPawn))))

(event Custom|OnTimerElasped
  (bind _index (Variables|Default|GetIndex))
  (Utilities|FlowControl|DoOnce false) ; enters at Reset
)

(event Custom|PrintEverythingDeviceRelated
  (bind (_outusers _returnvalue) (Class|InputDeviceLibrary|GetAllActiveUsers))
  (Development|PrintString (Utilities|String|Append (Utilities|String|ToString(Integer) _returnvalue) " active users"))
  (for _array_element _outusers
    (bind (_outinputdevices _returnvalue_2) (Class|InputDeviceLibrary|GetAllInputDevicesforUser _array_element))
    (Development|PrintString (Utilities|String|Append "User " (Utilities|String|ToString(Integer) _array_element) " has " (Utilities|String|ToString(Integer) _returnvalue_2) " devices:"))
    (for _array_element_2 _outinputdevices
      (Development|PrintString (Utilities|String|Append "-" (Utilities|String|ToString(Integer) _array_element_2)))
      (bind _returnvalue_3 (Class|InputDeviceLibrary|GetAllInputDevices))
      (Development|PrintString (Utilities|String|Append "Device count: " (Utilities|String|ToString(Integer) _returnvalue_3))))))

(event Input|EnhancedActionEvents|EnhancedInputActionIA_MenuSelect
  (params (ActionValue :type Float%20%28double-precision%29) (ElapsedSeconds :type Float%20%28double-precision%29) (TriggeredSeconds :type Float%20%28double-precision%29) (InputAction :type Input%20Action%20Object%20Reference :default "/Game/CouchGame2025/Input/Inputs/IA_MenuSelect.IA_MenuSelect")))

(event Input|EnhancedActionEvents|EnhancedInputActionIA_MenuSelect
  (params (ActionValue :type Float%20%28double-precision%29) (ElapsedSeconds :type Float%20%28double-precision%29) (TriggeredSeconds :type Float%20%28double-precision%29) (InputAction :type Input%20Action%20Object%20Reference :default "/Game/CouchGame2025/Input/Inputs/IA_MenuSelect.IA_MenuSelect"))
  (bind _index (Variables|Default|GetIndex))
  (Utilities|FlowControl|DoOnce false
    (:Completed
      (Utilities|IsValid (Variables|Default|GetCharacter%20Selection%20Widget)
        (:Is%20Valid
          _)
        (:Is%20Not%20Valid
          (Variables|Default|SetCharacter%20Selection%20Widget (Variables|/Game/CouchGame2025/Blueprint/Global/GM_CouchGame2025.GM_CouchGame2025_C|GetCharacterSelectionWidget (Variables|Default|GetGameMode)))))
      (Default|ProcessInput (Variables|Default|GetCharacter%20Selection%20Widget) ActionValue _index)
      (Utilities|Time|SetTimerbyEvent (delegate Custom|OnTimerElasped) 0.5)
      (Development|PrintString (Utilities|String|Append "Process menu input in " (Utilities|GetDisplayName self) " with player index " (Utilities|String|ToString(Integer) _index))))))

(event EventTick
  (params (DeltaSeconds :type Float%20%28single-precision%29)))

(event EventBeginPlay
  (bind _asgm_couch_game_2025 (Utilities|Casting|CastToGM_CouchGame2025 (Game|GetGameMode)))
  (Variables|Default|SetGameMode _asgm_couch_game_2025)
  (Variables|Default|SetLocal%20Multiplayer%20Settings (Variables|/Script/MultiplayerModule.LocalMultiplayerSubsystem|GetLocalMultiplayerSettings (Subsystems|GetLocalMultiplayerSubsystem)))
  (bind _index (Utilities|FlowControl|ForLoopwithBreak 0 (Class|GameplayStatics|GetNumPlayerControllers) :!label _label)
    (:LoopBody
      (if (== (Game|GetPlayerController _index) self)
        (Variables|Default|SetIndex _index)
        (goto _label Break)))))

(fn ConstructionScript)