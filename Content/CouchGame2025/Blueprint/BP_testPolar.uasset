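; BP_testPolar is a test child Blueprint that keeps its camera component oriented relative to the world origin.
; After running the parent Tick, it sets the camera's world rotation to the look-at rotation from the actor's location to (0,0,0).
; InvertLookAt switches this to the negated rotator.
; The custom event CE_AllowMovement sets the CanMove flag to true.
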(event Custom|CE_AllowMovement
  (Variables|Default|SetcanMove true))

(event EventTick
  (params (DeltaSeconds :type Float%20%28single-precision%29))
  (bind _returnvalue (Transformation|GetActorLocation))
  (bind _returnvalue_2 (Math|Vector|MakeVector 0.0 0.0 0.0))
  (bind _returnvalue_3 (Math|Rotator|FindLookatRotation _returnvalue _returnvalue_2))
  (|CallParentFunction DeltaSeconds)
  (Transformation|SetWorldRotation (Variables|Default|GetCameraComponent) (select (Variables|Default|GetInvertLookAt) (Class|KismetMathLibrary|NegateRotator _returnvalue_3) _returnvalue_3) false false))

(fn ConstructionScript)