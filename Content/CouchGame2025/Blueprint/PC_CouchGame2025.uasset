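; Player controller for CouchGame2025 that currently serves mainly to debug input device connections for local play.
; BeginPlay caches the game mode's character selection widget and binds to the game instance's input device connection change event.
; On each change it prints the changed device ID, then every device's class name, hardware ID, device type and connection state.
; The menu select input is an empty stub, and Tick does nothing.
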(event Custom|OnInputDeviceConnectionChange
  (params (NewConnectionState :type EInputDeviceConnectionState%20Enum :default "Invalid") (PlatformUserId :type Platform%20User%20Id%20Structure) (InputDeviceId :type Input%20Device%20Id%20Structure))
  (Development|PrintString (Utilities|String|ToString(Integer) InputDeviceId) true true "(R=0.000000,G=1.000000,B=0.020389,A=1.000000)")
  (bind _outinputdevices (Class|InputDeviceLibrary|GetAllInputDevices))
  (for _array_element _outinputdevices
    (bind _returnvalue (Class|InputDeviceLibrary|GetInputDeviceConnectionState _array_element))
    (Development|PrintString (Utilities|String|Append "Append Class Name - " (Utilities|String|ToString(Name) (.InputClassName (Utilities|Struct|BreakHardwareDeviceIdentifier (Class|InputDeviceSubsystem|GetInputDeviceHardwareIdentifier (|InputDeviceSubsystem) _array_element)))) " 
HW Device ID - " (Utilities|String|ToString(Name) (.HardwareDeviceIdentifier (Utilities|Struct|BreakHardwareDeviceIdentifier (Class|InputDeviceSubsystem|GetInputDeviceHardwareIdentifier (|InputDeviceSubsystem) _array_element)))) " 
primary device type" (Utilities|String|EnumtoString _returnvalue) " 
Connection State" (Utilities|String|EnumtoString (.PrimaryDeviceType (Utilities|Struct|BreakHardwareDeviceIdentifier (Class|InputDeviceSubsystem|GetInputDeviceHardwareIdentifier (|InputDeviceSubsystem) _array_element))))) true true "(R=0.000000,G=0.660000,B=1.000000,A=1.000000)" 1e+03)))

(event Input|EnhancedActionEvents|EnhancedInputActionIA_MenuSelect
  (params (ActionValue :type Float%20%28double-precision%29) (ElapsedSeconds :type Float%20%28double-precision%29) (TriggeredSeconds :type Float%20%28double-precision%29) (InputAction :type Input%20Action%20Object%20Reference :default "/Game/CouchGame2025/Input/Inputs/IA_MenuSelect.IA_MenuSelect")))

(event EventTick
  (params (DeltaSeconds :type Float%20%28single-precision%29)))

(event EventBeginPlay
  (bind _asbp_couch_game_2025game_mode (Utilities|Casting|CastToBP_CouchGame2025GameMode (Game|GetGameMode)))
  (Variables|Default|SetCharacter%20Selection%20Widget (Variables|/Game/CouchGame2025/Blueprint/Global/BP_CouchGame2025GameMode.BP_CouchGame2025GameMode_C|GetCharacterSelectionWidget _asbp_couch_game_2025game_mode))
  (EventDispatchers|BindEventtoOnInputDeviceConnectionChange (Game|GetGameInstance) (EventDispatchers|CreateEvent :!event Custom|OnInputDeviceConnectionChange)))

(fn ConstructionScript)